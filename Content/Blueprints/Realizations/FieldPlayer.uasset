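; FieldPlayer is the player-side field Blueprint that restores saved gold and opens the pause menu.
; On BeginPlay it loads the GRPGSaveGame from slot "A", if one exists, and copies only its Gold into the GRPG game instance.
; Releasing P pauses the game, then creates a PauseUI widget targeting the first party member and adds it to the viewport.
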(event EventBeginPlay
  (bind _returnvalue (SaveGame|DoesSaveGameExist "A"))
  (if _returnvalue
    (bind _returnvalue_2 (SaveGame|LoadGamefromSlot "A"))
    (bind _asgrpgsave_game (Utilities|Casting|CastToGRPGSaveGame _returnvalue_2))
    (bind _output_get (Variables|Default|Setload _asgrpgsave_game))
    (Variables|/Game/Blueprints/GRPGGameInstance.GRPGGameInstance_C|Setgold (CallFunction|GetGameGRPGInstance) (Variables|/Game/Blueprints/GRPGSaveGame.GRPGSaveGame_C|Getgold _output_get))))

(event Collision|EventActorBeginOverlap
  (params (OtherActor :type Actor%20Object%20Reference)))

(event EventTick
  (params (DeltaSeconds :type Float%20%28single-precision%29)))

(event Input|KeyboardEvents|P
  (params (Key :type Key%20Structure :default "None"))
  (:Released
    (Game|SetGamePaused true)
    (bind _returnvalue (UserInterface|CreateWidget "/Game/Views/Pause/PauseUI.PauseUI_C"))
    (Variables|/Game/Views/Pause/PauseUI.PauseUI_C|SetcharacterTrget _returnvalue (Utilities|Array|Get(acopy) (Variables|/Game/Blueprints/GRPGGameInstance.GRPGGameInstance_C|Getparty (CallFunction|GetGameGRPGInstance))))
    (UserInterface|Viewport|AddtoViewport _returnvalue 0)))

(fn ConstructionScript
  (|CallParentFunction))
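; MockDecisionMaker is a placeholder decision maker that picks a combat action for a character.
; On begin, it prints the character's name, asks the character to select a target, and assigns it a newly constructed MockCombatAction aimed at that target.
; MakeDicision then counts down a one-second delay using DeltaSeconds and returns true once it expires, simulating thinking time.
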(event EventBeginMakeDecision
  (params (character :type Game%20Character%20Object%20Reference))
  (Development|PrintString 0 (Utilities|String|Append (Variables|/Game/Models/GameCharacter.GameCharacter_C|GetcharacterName character) " make dicision."))
  (bind _target (Default|SelectTarget character))
  (bind _returnvalue (Game|ConstructObjectfromClass "/Game/Blueprints/Realizations/MockCombatAction.MockCombatAction_C" character _target))
  (Variables|/Game/Models/GameCharacter.GameCharacter_C|SetcombatAction character _returnvalue)
  (Variables|Default|SetdelayTimer 1.0))

(fn MakeDicision
  (params (deltaSeconds :type Float%20%28single-precision%29))
  (bind _output_get (Variables|Default|SetdelayTimer (- (Variables|Default|GetdelayTimer) deltaSeconds)))
  (return (<= _output_get 0.0)))
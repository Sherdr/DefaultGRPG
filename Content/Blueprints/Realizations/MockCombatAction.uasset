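; Mock combat action that makes a character perform a simple placeholder attack on its target.
; BeginExecuteAction asks the character for a new target if the current one has no HP left, then prints the attack, subtracts fixed damage and starts a short delay timer.
; ExecuteAction counts that timer down by delta seconds and returns true once it expires, signalling that the action is finished.
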(event EventBeginExecuteAction
  (params (character :type Game%20Character%20Object%20Reference))
  (bind _output_get (Variables|Default|Setcharacter character))
  (if (<= (Variables|/Game/Models/GameCharacter.GameCharacter_C|GetcurrentHP (Variables|Default|Gettarget)) 0)
    (bind _target (Default|SelectTarget _output_get))
    (Variables|Default|Settarget _target))
  (Utilities|IsValid (Variables|Default|Gettarget)
    (:Is%20Valid
      (Development|PrintString 0 (Utilities|String|Append (Variables|/Game/Models/GameCharacter.GameCharacter_C|GetcharacterName (Variables|Default|Getcharacter)) " attacks " (Variables|/Game/Models/GameCharacter.GameCharacter_C|GetcharacterName (Variables|Default|Gettarget))))
      (Variables|/Game/Models/GameCharacter.GameCharacter_C|SetcurrentHP (Variables|Default|Gettarget) (- (Variables|/Game/Models/GameCharacter.GameCharacter_C|GetcurrentHP (Variables|Default|Gettarget)) 10))
      (Variables|Default|SetdelayTimer 1.0))))

(fn ExecuteAction
  (params (deltaSeconds :type Float%20%28single-precision%29))
  (bind _output_get (Variables|Default|SetdelayTimer (- (Variables|Default|GetdelayTimer) deltaSeconds)))
  (return (<= _output_get 0.0)))
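; GRPGCameraComponent is a component that acts as a fixed-angle follow camera for the Pawn that owns it.
; Each tick it places itself Distance units back from the pawn's location along the forward vector of its Pitch angle.
; It sets its world rotation to that pitch with zero yaw and roll, so the view ignores the pawn's rotation.
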(event EventBeginPlay)

(event EventTick
  (params (DeltaSeconds :type Float%20%28single-precision%29))
  (bind _pitch (Variables|CameraProperties|Getpitch))
  (bind _returnvalue (Math|Rotator|MakeRotator 0.0 _pitch 0.0))
  (bind _aspawn (Utilities|Casting|CastToPawn (Components|GetOwner)))
  (bind _output_get (Variables|Default|Setlocation (Transformation|GetActorLocation _aspawn)))
  (Transformation|SetWorldLocationAndRotation (- _output_get (* (Math|Rotator|GetRotationXVector _returnvalue) (Variables|CameraProperties|Getdistance))) _returnvalue false false))
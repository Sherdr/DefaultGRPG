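; RPG game mode that initializes the game instance and starts a test combat on BeginPlay.
; It builds an enemy from a data table, creates a CombatEngine with both parties, and makes the combat UI each player character's decision maker.
; Tick drives the engine; when it reports completion, a DoOnce handles Game Over (reset, game-over screen) or Victory (award gold, remove UI, re-enable the player controller's tick, paused during combat).
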(event Custom|TestCombat
  (bind _returnvalue (Utilities|GetDataTableRow "/Game/Repositories/EnemiesList.EnemiesList" "s1")
    (:then
      (bind _return (CallFunction|CreateEnemyCharacter _returnvalue))
      (Utilities|Array|Add (Variables|Default|GetenemyParty) _return)
      (Actor|Tick|SetActorTickEnabled (Game|GetPlayerController 0))
      (bind _asgrpggame_instance (Utilities|Casting|CastToGRPGGameInstance (Game|GetGameInstance)))
      (bind _output_get (Variables|Default|SetplayerParty (Variables|/Game/Blueprints/GRPGGameInstance.GRPGGameInstance_C|Getparty _asgrpggame_instance)))
      (bind _returnvalue_2 (Game|ConstructObjectfromClass "/Game/Blueprints/CombatEngine.CombatEngine_C" self _output_get (Variables|Default|GetenemyParty)))
      (bind _output_get_2 (Variables|Default|SetcurrentCombatInstance _returnvalue_2))
      (Default|Construct _output_get_2)
      (bind _returnvalue_3 (UserInterface|CreateWidget (Variables|Default|GetcombatUIclass)))
      (bind _output_get_3 (Variables|Default|SetcombatUI _returnvalue_3))
      (UserInterface|Viewport|AddtoViewport _output_get_3 0)
      (for _array_element (Variables|Default|GetplayerParty)
        (Default|AddPlayerCharacterPanel (Variables|Default|GetcombatUI) _array_element)
        (Variables|/Game/Models/GameCharacter.GameCharacter_C|SetdecisionMaker _array_element (Variables|Default|GetcombatUI)))
      (for _array_element_2 (Variables|Default|GetenemyParty)
        (Default|AddEnemyCharacterPanel (Variables|Default|GetcombatUI) _array_element_2)))))

(event EventBeginPlay
  (bind _asgrpggame_instance (Utilities|Casting|CastToGRPGGameInstance (Game|GetGameInstance)))
  (Default|Init _asgrpggame_instance)
  (CallFunction|TestCombat))

(event EventTick
  (params (DeltaSeconds :type Float%20%28single-precision%29))
  (bind _asgrpggame_instance (CallFunction|GetGameGRPGInstance))
  (bind _currentcombatinstance (Variables|Default|GetcurrentCombatInstance))
  (Utilities|IsValid _currentcombatinstance
    (:Is%20Valid
      (bind _iscombatover (Default|Tick _currentcombatinstance DeltaSeconds))
      (if _iscombatover
        (Utilities|FlowControl|DoOnce false
          (:Completed
            (switch Utilities|FlowControl|Switch|SwitchonCombatPhase (Variables|/Game/Blueprints/CombatEngine.CombatEngine_C|Getphase (Variables|Default|GetcurrentCombatInstance))
              (:NewEnumerator2
                (Default|PrepareReset (CallFunction|GetGameGRPGInstance))
                (Widget|RemovefromParent (Variables|Default|GetcombatUI))
                (Variables|Default|SetcombatUI 0)
                (bind _returnvalue (UserInterface|CreateWidget (Variables|Default|GetgameOverUIclass)))
                (UserInterface|Viewport|AddtoViewport _returnvalue 0))
              (:NewEnumerator3
                (Variables|/Game/Blueprints/GRPGGameInstance.GRPGGameInstance_C|Setgold _asgrpggame_instance (+ (Variables|/Game/Blueprints/CombatEngine.CombatEngine_C|GetgoldTotal (Variables|Default|GetcurrentCombatInstance)) (Variables|/Game/Blueprints/GRPGGameInstance.GRPGGameInstance_C|Getgold _asgrpggame_instance)))
                (Actor|Tick|SetActorTickEnabled (Game|GetPlayerController 0) true)
                (for _array_element (Variables|Default|GetplayerParty)
                  (Variables|/Game/Models/GameCharacter.GameCharacter_C|SetdecisionMaker _array_element 0)
                  (Widget|RemovefromParent (Variables|Default|GetcombatUI))
                  (Variables|Default|SetcombatUI 0)
                  (Utilities|Array|Clear (Variables|Default|GetenemyParty)))))))))))

(fn ConstructionScript)
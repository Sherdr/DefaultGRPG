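; CombatEngine runs turn-based combat between a player party and an enemy party, combined into one combatant order.
; Its Tick function alternates Decision and Action phases, polling each living combatant until it finishes deciding or executing, then moving to the next.
; After each full pass it checks whether either party is entirely dead, entering GameOver or Victory, where Tick returns true.
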(event Custom|SetPhase
  (params (phase :type CombatPhase%20Enum :default "NewEnumerator0"))
  (bind _output_get (Variables|Default|Setphase phase))
  (switch Utilities|FlowControl|Switch|SwitchonCombatPhase _output_get
    (:NewEnumerator0
      _)
    (:NewEnumerator1
      _))
  (Variables|Default|SettickTargetIndex 0)
  (CallFunction|SelectNextCharacter))

(event Custom|SelectNextCharacter
  (bind _combatantorder (Variables|Default|GetcombatantOrder))
  (Variables|Default|SetwaitingCharacter false)
  (bind _index (Utilities|FlowControl|ForLoopwithBreak (Variables|Default|GettickTargetIndex) (- (Utilities|Array|Length _combatantorder) 1) :!label _label)
    (:LoopBody
      (if (Utilities|Array|IsValidIndex _combatantorder _index)
        (bind _output_get (Variables|Default|Setcharacter (Utilities|Array|Get(acopy) _combatantorder _index)))
        (if (> (Variables|/Game/Models/GameCharacter.GameCharacter_C|GetcurrentHP _output_get) 0)
          (Variables|Default|SettickTargetIndex (+ _index 1))
          (Variables|Default|SetcurentTickTarget (Variables|Default|Getcharacter))
          (goto _label Break))))
    (:Completed
      (if (not (Utilities|Array|IsValidIndex _combatantorder _index))
        (Variables|Default|SettickTargetIndex -1)
        (Variables|Default|SetcurentTickTarget 0)))))

(event Custom|Construct
  (Utilities|Array|AppendArray (Variables|Default|GetcombatantOrder) (Variables|Default|GetplayerParty))
  (Utilities|Array|AppendArray (Variables|Default|GetcombatantOrder) (Variables|Default|GetenemyParty))
  (for _array_element (Variables|Default|GetcombatantOrder)
    (Variables|/Game/Models/GameCharacter.GameCharacter_C|SetcombatInstance _array_element self)
    (Variables|Default|SettickTargetIndex 0)
    (CallFunction|SetPhase "NewEnumerator0")))

(event Custom|Destruct
  (Utilities|Array|Clear (Variables|Default|GetenemyParty))
  (Utilities|Array|Clear (Variables|Default|GetcombatantOrder)))

(fn Tick
  (params (deltaSeconds :type Float%20%28single-precision%29))
  (switch Utilities|FlowControl|Switch|SwitchonCombatPhase (Variables|Default|Getphase)
    (:NewEnumerator0
      (if (Variables|Default|GetwaitingCharacter)
        (bind _return (Default|MakeDecision (Variables|Default|GetcurentTickTarget) deltaSeconds))
        (if _return
          (CallFunction|SelectNextCharacter)
          (if (== (Variables|Default|GettickTargetIndex) -1)
            (CallFunction|SetPhase "NewEnumerator1")
            (bind _isgameover (CallFunction|CheckGameOver :!label _label))
            (if _isgameover
              (CallFunction|SetPhase "NewEnumerator2")
              (else
                (bind _isvictory (CallFunction|CheckVictory))
                (if _isvictory
                  (CallFunction|SetPhase "NewEnumerator3"))))
            (return false)))
        (else
          (Default|BeginMakeDecision (Variables|Default|GetcurentTickTarget))
          (Variables|Default|SetwaitingCharacter true))))
    (:NewEnumerator1
      (if (Variables|Default|GetwaitingCharacter)
        (bind _return_2 (Default|ExecuteAction (Variables|Default|GetcurentTickTarget) deltaSeconds))
        (if _return_2
          (CallFunction|SelectNextCharacter)
          (if (== (Variables|Default|GettickTargetIndex) -1)
            (CallFunction|SetPhase "NewEnumerator0")
            (goto _label)))
        (else
          (Default|BeginExecuteAction (Variables|Default|GetcurentTickTarget))
          (Variables|Default|SetwaitingCharacter true))))
    (:NewEnumerator2
      (return true))
    (:NewEnumerator3
      (return true))))

(fn CheckGameOver
  (Variables|Default|SetdeadCount 0)
  (for _array_element (Variables|Default|GetplayerParty)
    (if (<= (Variables|/Game/Models/GameCharacter.GameCharacter_C|GetcurrentHP _array_element) 0)
      (Math|Integer|IncrementInt (Variables|Default|GetdeadCount))))
  (return (== (Variables|Default|GetdeadCount) (Utilities|Array|Length (Variables|Default|GetplayerParty)))))

(fn CheckVictory
  (Variables|Default|SetdeadCount 0)
  (for _array_element (Variables|Default|GetenemyParty)
    (if (<= (Variables|/Game/Models/GameCharacter.GameCharacter_C|GetcurrentHP _array_element) 0)
      (Math|Integer|IncrementInt (Variables|Default|GetdeadCount))))
  (return (== (Variables|Default|GetdeadCount) (Utilities|Array|Length (Variables|Default|GetenemyParty)))))
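; GRPGGameInstance is the RPG game instance that holds the player's Party.
; On Init, guarded by an IsInitialized flag, it reads the "s1" row from the CharactersList data table, creates a player character from it and adds it to the Party if valid.
; PrepareReset clears the flag and empties the Party, so a later Init can rebuild it.
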(event Custom|PrepareReset
  (Variables|Default|SetisInitialized false)
  (Utilities|Array|Clear (Variables|GameData|Getparty)))

(event Custom|Init
  (if (not (Variables|Default|GetisInitialized))
    (Variables|Default|SetisInitialized true)
    (bind _returnvalue (Utilities|GetDataTableRow "/Game/Repositories/CharactersList.CharactersList" "s1")
      (:then
        (bind _return (CallFunction|CreatePlayerCharacter _returnvalue))
        (Utilities|IsValid _return
          (:Is%20Valid
            (Utilities|Array|Add (Variables|GameData|Getparty) _return)))))))

(event EventInit
  (if (not (Variables|Default|GetisInitialized))
    (Variables|Default|SetisInitialized true)
    (bind _returnvalue (Utilities|GetDataTableRow "/Game/Repositories/CharactersList.CharactersList" "s1")
      (:then
        (bind _return (CallFunction|CreatePlayerCharacter _returnvalue))
        (Utilities|IsValid _return
          (:Is%20Valid
            (Utilities|Array|Add (Variables|GameData|Getparty) _return)))))))
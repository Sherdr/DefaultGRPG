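; ConstructGameCharacter is a factory that builds GameCharacter objects for players and enemies, outered to CharactersList.
; CreatePlayerCharacter looks up the ClassId row in the ClassesList data table and seeds name, class info and starting stats, returning the character only when the row is found.
; CreateEnemyCharacter copies stats straight from the supplied enemy info, zeroes MP and attaches a MockDecisionMaker as its decision maker.
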(fn CreatePlayerCharacter
  (params (characterInfo :type Character%20Info%20Structure))
  (bind (_charactername _classid) (Utilities|Struct|BreakCharacterInfo characterInfo))
  (bind _returnvalue (Game|ConstructObjectfromClass "/Game/Models/GameCharacter.GameCharacter_C" "/Game/Repositories/CharactersList.CharactersList" true))
  (LocalVariables|Setcharacter _returnvalue)
  (bind _returnvalue_2 (Utilities|GetDataTableRow "/Game/Repositories/ClassesList.ClassesList" _classid)
    (:then
      (bind _output_get (Variables|/Game/Models/GameCharacter.GameCharacter_C|SetclassInfo (LocalVariables|Getcharacter) _returnvalue_2))
      (Variables|/Game/Models/GameCharacter.GameCharacter_C|SetcharacterName (LocalVariables|Getcharacter) _charactername)
      (Variables|/Game/Models/GameCharacter.GameCharacter_C|SetcurrentHP (LocalVariables|Getcharacter) (.startmaxhp (Utilities|Struct|BreakClassInfo _output_get)))
      (Variables|/Game/Models/GameCharacter.GameCharacter_C|SetmaxHP (LocalVariables|Getcharacter) (.startmaxhp (Utilities|Struct|BreakClassInfo _output_get)))
      (Variables|/Game/Models/GameCharacter.GameCharacter_C|SetcurrentMP (LocalVariables|Getcharacter) (.startmaxmp (Utilities|Struct|BreakClassInfo _output_get)))
      (Variables|/Game/Models/GameCharacter.GameCharacter_C|SetmaxMP (LocalVariables|Getcharacter) (.startmaxmp (Utilities|Struct|BreakClassInfo _output_get)))
      (Variables|/Game/Models/GameCharacter.GameCharacter_C|Setattack (LocalVariables|Getcharacter) (.startattack (Utilities|Struct|BreakClassInfo _output_get)))
      (Variables|/Game/Models/GameCharacter.GameCharacter_C|Setdefense (LocalVariables|Getcharacter) (.startdefense (Utilities|Struct|BreakClassInfo _output_get)))
      (Variables|/Game/Models/GameCharacter.GameCharacter_C|Setluck (LocalVariables|Getcharacter) (.startluck (Utilities|Struct|BreakClassInfo _output_get)))
      (return (LocalVariables|Getcharacter)))))

(fn CreateEnemyCharacter
  (params (enemuInfo :type Enemy%20Info%20Structure))
  (bind (_enemyname _hp _atk _def _lck) (Utilities|Struct|BreakEnemyInfo enemuInfo))
  (bind _returnvalue (Game|ConstructObjectfromClass "/Game/Models/GameCharacter.GameCharacter_C" "/Game/Repositories/CharactersList.CharactersList"))
  (bind _output_get (LocalVariables|Setcharacter _returnvalue))
  (Variables|/Game/Models/GameCharacter.GameCharacter_C|SetcharacterName _output_get _enemyname)
  (Variables|/Game/Models/GameCharacter.GameCharacter_C|SetcurrentHP _output_get _hp)
  (Variables|/Game/Models/GameCharacter.GameCharacter_C|SetmaxHP _output_get _hp)
  (Variables|/Game/Models/GameCharacter.GameCharacter_C|SetcurrentMP _output_get 0)
  (Variables|/Game/Models/GameCharacter.GameCharacter_C|SetmaxMP _output_get 0)
  (Variables|/Game/Models/GameCharacter.GameCharacter_C|Setattack _output_get _atk)
  (Variables|/Game/Models/GameCharacter.GameCharacter_C|Setdefense _output_get _def)
  (Variables|/Game/Models/GameCharacter.GameCharacter_C|Setluck _output_get _lck)
  (bind _returnvalue_2 (Game|ConstructObjectfromClass "/Game/Blueprints/Realizations/MockDecisionMaker.MockDecisionMaker_C" (LocalVariables|Getcharacter)))
  (Variables|/Game/Models/GameCharacter.GameCharacter_C|SetdecisionMaker (LocalVariables|Getcharacter) _returnvalue_2)
  (return (LocalVariables|Getcharacter)))